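; PC-Water, likely a player controller for a water level, gives the player's diver a hold-to-thrust jetpack.
; BeginPlay caches the first BPPlayer1 found in the level, and the Enhanced Input jump action sets and clears a jetpack flag.
; While the flag is set, Tick applies a constant upward force to the Diver component at the world origin rather than at the body's position.
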(event Input|EnhancedActionEvents|EnhancedInputActionIA-Jump
  (params (ActionValue :type Boolean) (ElapsedSeconds :type Float%20%28double-precision%29) (TriggeredSeconds :type Float%20%28double-precision%29) (InputAction :type Input%20Action%20Object%20Reference :default "/Game/Input/actions/IA-Jump.IA-Jump"))
  (:Triggered
    (Variables|Default|SetJectpack%20is%20active true))
  (:Completed
    (Variables|Default|SetJectpack%20is%20active false)))

(event EventBeginPlay
  (bind _outactors (Actor|GetAllActorsOfClass "/Game/Blueprint/BP-Player1.BP-Player1_C"))
  (Variables|Default|SetBP-Player1 (Utilities|Array|Get(acopy) _outactors)))

(event EventTick
  (params (DeltaSeconds :type Float%20%28single-precision%29))
  (if (Variables|Default|GetJectpack%20is%20active)
    (Utilities|IsValid (Variables|Default|GetBP-Player1)
      (:Is%20Valid
        (Class|PrimitiveComponent|AddForceatLocation (Variables|/Game/Blueprint/BP-Player1.BP-Player1_C|GetDiver (Variables|Default|GetBP-Player1)) "0.000000,0.000000,50.000000" "0.000000,0.000000,0.000000" "None")))))

(fn ConstructionScript)